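; TV actor that, while IsActive is set, repositions itself on Tick from ReturnWorldLocationAndRotation.
; A 0.25-second Delay then clears IsActive, so each activation yields only a brief window of movement.
; The function holds math for placing it DistanceToPlayer ahead of the VR_Home camera's yaw, turned toward it with a 90-degree offset, but those nodes appear unconnected.
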(event `self.ReceiveTick`
  (params (DeltaSeconds :type "Float (single-precision)"))
  (bind _camera (`/Game/Blueprints/VR_Home.Camera` (cast `/Game/Blueprints/VR_Home` (`GameplayStatics.GetPlayerPawn` 0) :!pure true)))
  (bind (_returnvalue_roll _returnvalue_pitch _returnvalue_yaw) (`KismetMathLibrary.BreakRotator` (`SceneComponent.K2_GetComponentRotation` _camera)))
  (bind _returnvalue (`SceneComponent.K2_GetComponentLocation` _camera))
  (bind (_returnvalue_roll_2 _returnvalue_pitch_2 _returnvalue_yaw_2) (`KismetMathLibrary.BreakRotator` (`KismetMathLibrary.FindLookAtRotation` (`self.K2_GetActorLocation`) _returnvalue)))
  (if (`self.isActive`)
    (`self.K2_SetActorLocationAndRotation` (+ (* (`KismetMathLibrary.GetForwardVector` (`KismetMathLibrary.MakeRotator` 0.0 0.0 _returnvalue_yaw)) (`self.DistanceToPlayer`)) _returnvalue) (`KismetMathLibrary.MakeRotator` 0.0 0.0 (+ _returnvalue_yaw_2 90.0)))
    (`KismetSystemLibrary.Delay` 0.25)
    (set `self.isActive` false)))

(fn `UserConstructionScript`)