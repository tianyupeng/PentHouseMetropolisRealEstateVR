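; MyLib provides a TraceForTeleport helper that aims a beam for teleporting and validates the destination.
; While the teleport button is held, it line-traces forward from an arrow component and stretches the particle beam to the hit point or trace end.
; It returns the hit location and allows teleporting only if the blocking actor is tagged "ground".
; Releasing the button hides the beam.
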(fn `TraceForTeleport`
  (params (Arrow :type "ArrowComponent Object Reference") (MyBeamTele :type "ParticleSystemComponent Object Reference") (IsHoldingTeleportBut :type Boolean) (`Cantele?` :type Boolean))
  (returns (`CanTeleport?1` :type Boolean) (Location :type "Vector Structure"))
  (locals (HoldingTele :type Boolean) (ArrowLeft :type "ArrowComponent Object Reference") (TeleBeam :type "ParticleSystemComponent Object Reference") (`CanTeleport?` :type Boolean))
  (bind _telebeam (`local.TeleBeam`))
  (bind _arrowleft (`local.ArrowLeft`))
  (bind _returnvalue (`SceneComponent.K2_GetComponentLocation` _arrowleft))
  (set `local.CanTeleport?` `Cantele?`)
  (set `local.ArrowLeft` Arrow)
  (set `local.TeleBeam` MyBeamTele)
  (set `local.HoldingTele` IsHoldingTeleportBut)
  (if (`local.HoldingTele`)
    (`SceneComponent.SetVisibility` _telebeam true true)
    (`ParticleSystemComponent.SetBeamSourcePoint` (`local.TeleBeam`) 0 _returnvalue 0)
    (bind _outhit (`KismetSystemLibrary.LineTraceSingle` (`local.__WorldContext`) _returnvalue (+ (* (`SceneComponent.GetForwardVector` _arrowleft) 100000.0) _returnvalue) "TraceTypeQuery3"))
    (bind (_bblockinghit _binitialoverlap _time _distance _location _impactpoint _normal _impactnormal _physmat _hitactor _hitcomponent _hitbonename _hititem _faceindex _tracestart _traceend) (`GameplayStatics.BreakHitResult` _outhit))
    (`ParticleSystemComponent.SetBeamTargetPoint` (`local.TeleBeam`) 0 (`KismetMathLibrary.SelectVector` _location _traceend _bblockinghit) 0)
    (if _bblockinghit
      (if (`Actor.ActorHasTag` _hitactor "ground")
        (set `local.CanTeleport?` true)
        (else
          (set `local.CanTeleport?` false :!label _label)))
      (else
        (goto _label)))
    (return (`local.CanTeleport?`) _location)
    (else
      (`SceneComponent.SetVisibility` _telebeam false true))))