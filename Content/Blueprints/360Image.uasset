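; VR 360-image picker that shows five spinning preview meshes above the VR_Home pawn's left hand, yawed toward the camera each tick.
; On BeginPlay it loads JPGs from Content/360Image into a texture array.
; Left/right events page by five with wraparound, swapping dynamic materials between scale timelines while player input is disabled.
; On360Image and Off360Image toggle the meshes' visibility and collision.
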(event `self.ReceiveTick`
  (params (DeltaSeconds :type "Float (single-precision)"))
  (bind _asvr_home (cast `/Game/Blueprints/VR_Home` (`GameplayStatics.GetPlayerPawn` 0) :!pure true))
  (`SceneComponent.K2_AddLocalRotation` (`self.StaticMesh`) (* (`KismetMathLibrary.MakeRotator` 0.0 0.0 (`self.RotateSpeed`)) DeltaSeconds) false false)
  (`SceneComponent.K2_AddLocalRotation` (`self.StaticMesh1`) (* (`KismetMathLibrary.MakeRotator` 0.0 0.0 (`self.RotateSpeed`)) DeltaSeconds) false false)
  (`SceneComponent.K2_AddLocalRotation` (`self.StaticMesh2`) (* (`KismetMathLibrary.MakeRotator` 0.0 0.0 (`self.RotateSpeed`)) DeltaSeconds) false false)
  (`SceneComponent.K2_AddLocalRotation` (`self.StaticMesh3`) (* (`KismetMathLibrary.MakeRotator` 0.0 0.0 (`self.RotateSpeed`)) DeltaSeconds) false false)
  (`SceneComponent.K2_AddLocalRotation` (`self.StaticMesh4`) (* (`KismetMathLibrary.MakeRotator` 0.0 0.0 (`self.RotateSpeed`)) DeltaSeconds) false false)
  (`self.K2_SetActorLocationAndRotation` (+ (`SceneComponent.K2_GetComponentLocation` (`/Game/Blueprints/VR_Home.LeftHand` _asvr_home)) (* (`self.GetActorUpVector` _asvr_home) 35.0)) (`KismetMathLibrary.MakeRotator` 0.0 0.0 (.yaw (`KismetMathLibrary.FindLookAtRotation` (`self.K2_GetActorLocation`) (`SceneComponent.K2_GetComponentLocation` (`/Game/Blueprints/VR_Home.Camera` _asvr_home)))))))

(event `self.ReceiveBeginPlay`
  (bind _returnvalue (`KismetStringLibrary.Concat_StrStr` (`GetProjectPath.GetProjectPath`) "Content/" "360Image/"))
  (set `self.360ImageDir` _returnvalue)
  (bind _output_get (set `self.Array360ImagePath` (`VictoryBPFunctionLibrary.JoyFileIO_GetFiles` _returnvalue "jpg")))
  (for _index (range (`KismetArrayLibrary.Array_Length` _output_get))
    (`KismetArrayLibrary.Array_Add` (`self.Texture360Array`) (`.ReturnValue` (`VictoryBPFunctionLibrary.Victory_LoadTexture2D_FromFile` (`VictoryBPFunctionLibrary.AppendMultiple` (`self.360ImageDir`) (`|GetArrayItem` (`self.Array360ImagePath`) _index)) "JPG"))))
  (`KismetSystemLibrary.PrintString` (`KismetStringLibrary.Conv_IntToString` (`KismetArrayLibrary.Array_Length` (`self.Texture360Array`))) true true (struct :`G` 0.66 :`B` 1.0 :`A` 1.0) 20.0))

(event `Change360MatRight`
  (`self.DisableInput` (`GameplayStatics.GetPlayerPawn` 0) (`GameplayStatics.GetPlayerController` 0))
  (`|ExecutionSequence`
    (:`then_0`
      (bind (_direction _scale) (`Timeline|Timeline_0` :!via `PlayFromStart`)
        (:`Update`
          (`SceneComponent.SetWorldScale3D` (`self.StaticMesh`) (`KismetMathLibrary.MakeVector` _scale _scale _scale)))
        (:`Finished`
          (if (>= (`self.StaticMesh_Mat`) (- (`KismetArrayLibrary.Array_Length` (`self.Texture360Array`)) 5))
            (set `self.StaticMesh_Mat` (- (+ (`self.StaticMesh_Mat`) 5) (`KismetArrayLibrary.Array_Length` (`self.Texture360Array`))))
            (else
              (set `self.StaticMesh_Mat` (+ (`self.StaticMesh_Mat`) 5))))
          (bind _returnvalue (`KismetMaterialLibrary.CreateDynamicMaterialInstance` "/Game/Videos/UI_VID_IMAGE/IMage/360/M_anh360_Inst.M_anh360_Inst"))
          (`MaterialInstanceDynamic.SetTextureParameterValue` _returnvalue "Image360" (`|GetArrayItem` (`self.Texture360Array`) (`self.StaticMesh_Mat`)))
          (`PrimitiveComponent.SetMaterial` (`self.StaticMesh`) 0 _returnvalue)
          (bind (_direction_2 _scale_2) (`Timeline|Timeline_1` :!via `PlayFromStart`)
            (:`Update`
              (`SceneComponent.SetWorldScale3D` (`self.StaticMesh`) (`KismetMathLibrary.MakeVector` _scale_2 _scale_2 _scale_2)))
            (:`Finished`
              (`self.EnableInput` (`GameplayStatics.GetPlayerPawn` 0) (`GameplayStatics.GetPlayerController` 0)))))))
    (:`then_1`
      (bind (_direction_3 _scale_3) (`Timeline|Timeline_2` :!via `PlayFromStart`)
        (:`Update`
          (`SceneComponent.SetWorldScale3D` (`self.StaticMesh1`) (`KismetMathLibrary.MakeVector` _scale_3 _scale_3 _scale_3)))
        (:`Finished`
          (if (>= (`self.StaticMesh1_Mat`) (- (`KismetArrayLibrary.Array_Length` (`self.Texture360Array`)) 5))
            (set `self.StaticMesh1_Mat` (- (+ (`self.StaticMesh1_Mat`) 5) (`KismetArrayLibrary.Array_Length` (`self.Texture360Array`))))
            (else
              (set `self.StaticMesh1_Mat` (+ (`self.StaticMesh1_Mat`) 5))))
          (bind _returnvalue_2 (`KismetMaterialLibrary.CreateDynamicMaterialInstance` "/Game/Videos/UI_VID_IMAGE/IMage/360/M_anh360_Inst.M_anh360_Inst"))
          (`MaterialInstanceDynamic.SetTextureParameterValue` _returnvalue_2 "Image360" (`|GetArrayItem` (`self.Texture360Array`) (`self.StaticMesh1_Mat`)))
          (`PrimitiveComponent.SetMaterial` (`self.StaticMesh1`) 0 _returnvalue_2)
          (bind (_direction_4 _scale_4) (`Timeline|Timeline_3` :!via `PlayFromStart`)
            (:`Update`
              (`SceneComponent.SetWorldScale3D` (`self.StaticMesh1`) (`KismetMathLibrary.MakeVector` _scale_4 _scale_4 _scale_4)))))))
    (:`then_2`
      (bind (_direction_5 _scale_5) (`Timeline|Timeline_4` :!via `PlayFromStart`)
        (:`Update`
          (`SceneComponent.SetWorldScale3D` (`self.StaticMesh2`) (`KismetMathLibrary.MakeVector` _scale_5 _scale_5 _scale_5)))
        (:`Finished`
          (if (>= (`self.StaticMesh2_Mat`) (- (`KismetArrayLibrary.Array_Length` (`self.Texture360Array`)) 5))
            (set `self.StaticMesh2_Mat` (- (+ (`self.StaticMesh2_Mat`) 5) (`KismetArrayLibrary.Array_Length` (`self.Texture360Array`))))
            (else
              (set `self.StaticMesh2_Mat` (+ (`self.StaticMesh2_Mat`) 5))))
          (bind _returnvalue_3 (`KismetMaterialLibrary.CreateDynamicMaterialInstance` "/Game/Videos/UI_VID_IMAGE/IMage/360/M_anh360_Inst.M_anh360_Inst"))
          (`MaterialInstanceDynamic.SetTextureParameterValue` _returnvalue_3 "Image360" (`|GetArrayItem` (`self.Texture360Array`) (`self.StaticMesh2_Mat`)))
          (`PrimitiveComponent.SetMaterial` (`self.StaticMesh2`) 0 _returnvalue_3)
          (bind (_direction_6 _scale_6) (`Timeline|Timeline_5` :!via `PlayFromStart`)
            (:`Update`
              (`SceneComponent.SetWorldScale3D` (`self.StaticMesh2`) (`KismetMathLibrary.MakeVector` _scale_6 _scale_6 _scale_6)))))))
    (:`then_3`
      (bind (_direction_7 _scale_7) (`Timeline|Timeline_6` :!via `PlayFromStart`)
        (:`Update`
          (`SceneComponent.SetWorldScale3D` (`self.StaticMesh3`) (`KismetMathLibrary.MakeVector` _scale_7 _scale_7 _scale_7)))
        (:`Finished`
          (if (>= (`self.StaticMesh3_Mat`) (- (`KismetArrayLibrary.Array_Length` (`self.Texture360Array`)) 5))
            (set `self.StaticMesh3_Mat` (- (+ (`self.StaticMesh3_Mat`) 5) (`KismetArrayLibrary.Array_Length` (`self.Texture360Array`))))
            (else
              (set `self.StaticMesh3_Mat` (+ (`self.StaticMesh3_Mat`) 5))))
          (bind _returnvalue_4 (`KismetMaterialLibrary.CreateDynamicMaterialInstance` "/Game/Videos/UI_VID_IMAGE/IMage/360/M_anh360_Inst.M_anh360_Inst"))
          (`MaterialInstanceDynamic.SetTextureParameterValue` _returnvalue_4 "Image360" (`|GetArrayItem` (`self.Texture360Array`) (`self.StaticMesh3_Mat`)))
          (`PrimitiveComponent.SetMaterial` (`self.StaticMesh3`) 0 _returnvalue_4)
          (bind (_direction_8 _scale_8) (`Timeline|Timeline_7` :!via `PlayFromStart`)
            (:`Update`
              (`SceneComponent.SetWorldScale3D` (`self.StaticMesh3`) (`KismetMathLibrary.MakeVector` _scale_8 _scale_8 _scale_8)))))))
    (:`then_4`
      (bind (_direction_9 _scale_9) (`Timeline|Timeline_8` :!via `PlayFromStart`)
        (:`Update`
          (`SceneComponent.SetWorldScale3D` (`self.StaticMesh4`) (`KismetMathLibrary.MakeVector` _scale_9 _scale_9 _scale_9)))
        (:`Finished`
          (if (>= (`self.StaticMesh4_Mat`) (- (`KismetArrayLibrary.Array_Length` (`self.Texture360Array`)) 5))
            (set `self.StaticMesh4_Mat` (- (+ (`self.StaticMesh4_Mat`) 5) (`KismetArrayLibrary.Array_Length` (`self.Texture360Array`))))
            (else
              (set `self.StaticMesh4_Mat` (+ (`self.StaticMesh4_Mat`) 5))))
          (bind _returnvalue_5 (`KismetMaterialLibrary.CreateDynamicMaterialInstance` "/Game/Videos/UI_VID_IMAGE/IMage/360/M_anh360_Inst.M_anh360_Inst"))
          (`MaterialInstanceDynamic.SetTextureParameterValue` _returnvalue_5 "Image360" (`|GetArrayItem` (`self.Texture360Array`) (`self.StaticMesh4_Mat`)))
          (`PrimitiveComponent.SetMaterial` (`self.StaticMesh4`) 0 _returnvalue_5)
          (bind (_direction_10 _scale_10) (`Timeline|Timeline_9` :!via `PlayFromStart`)
            (:`Update`
              (`SceneComponent.SetWorldScale3D` (`self.StaticMesh4`) (`KismetMathLibrary.MakeVector` _scale_10 _scale_10 _scale_10)))))))))

(event `Change360MatLeft`
  (`self.DisableInput` (`GameplayStatics.GetPlayerPawn` 0) (`GameplayStatics.GetPlayerController` 0))
  (`|ExecutionSequence`
    (:`then_0`
      (bind (_direction _scale) (`Timeline|Timeline_10` :!via `PlayFromStart`)
        (:`Update`
          (`SceneComponent.SetWorldScale3D` (`self.StaticMesh`) (`KismetMathLibrary.MakeVector` _scale _scale _scale)))
        (:`Finished`
          (if (<= (`self.StaticMesh_Mat`) 4)
            (set `self.StaticMesh_Mat` (+ (- (`self.StaticMesh_Mat`) 5) (`KismetArrayLibrary.Array_Length` (`self.Texture360Array`))))
            (else
              (set `self.StaticMesh_Mat` (- (`self.StaticMesh_Mat`) 5))))
          (bind _returnvalue (`KismetMaterialLibrary.CreateDynamicMaterialInstance` "/Game/Videos/UI_VID_IMAGE/IMage/360/M_anh360_Inst.M_anh360_Inst"))
          (`MaterialInstanceDynamic.SetTextureParameterValue` _returnvalue "Image360" (`|GetArrayItem` (`self.Texture360Array`) (`self.StaticMesh_Mat`)))
          (`PrimitiveComponent.SetMaterial` (`self.StaticMesh`) 0 _returnvalue)
          (bind (_direction_2 _scale_2) (`Timeline|Timeline_11` :!via `PlayFromStart`)
            (:`Update`
              (`SceneComponent.SetWorldScale3D` (`self.StaticMesh`) (`KismetMathLibrary.MakeVector` _scale_2 _scale_2 _scale_2)))
            (:`Finished`
              (`self.EnableInput` (`GameplayStatics.GetPlayerPawn` 0) (`GameplayStatics.GetPlayerController` 0)))))))
    (:`then_1`
      (bind (_direction_3 _scale_3) (`Timeline|Timeline_12` :!via `PlayFromStart`)
        (:`Update`
          (`SceneComponent.SetWorldScale3D` (`self.StaticMesh1`) (`KismetMathLibrary.MakeVector` _scale_3 _scale_3 _scale_3)))
        (:`Finished`
          (if (<= (`self.StaticMesh1_Mat`) 4)
            (set `self.StaticMesh1_Mat` (+ (`KismetArrayLibrary.Array_Length` (`self.Texture360Array`)) (- (`self.StaticMesh1_Mat`) 5)))
            (else
              (set `self.StaticMesh1_Mat` (- (`self.StaticMesh1_Mat`) 5))))
          (bind _returnvalue_2 (`KismetMaterialLibrary.CreateDynamicMaterialInstance` "/Game/Videos/UI_VID_IMAGE/IMage/360/M_anh360_Inst.M_anh360_Inst"))
          (`MaterialInstanceDynamic.SetTextureParameterValue` _returnvalue_2 "Image360" (`|GetArrayItem` (`self.Texture360Array`) (`self.StaticMesh1_Mat`)))
          (`PrimitiveComponent.SetMaterial` (`self.StaticMesh1`) 0 _returnvalue_2)
          (bind (_direction_4 _scale_4) (`Timeline|Timeline_13` :!via `PlayFromStart`)
            (:`Update`
              (`SceneComponent.SetWorldScale3D` (`self.StaticMesh1`) (`KismetMathLibrary.MakeVector` _scale_4 _scale_4 _scale_4)))))))
    (:`then_2`
      (bind (_direction_5 _scale_5) (`Timeline|Timeline_14` :!via `PlayFromStart`)
        (:`Update`
          (`SceneComponent.SetWorldScale3D` (`self.StaticMesh2`) (`KismetMathLibrary.MakeVector` _scale_5 _scale_5 _scale_5)))
        (:`Finished`
          (if (<= (`self.StaticMesh2_Mat`) 4)
            (set `self.StaticMesh2_Mat` (+ (- (`self.StaticMesh2_Mat`) 5) (`KismetArrayLibrary.Array_Length` (`self.Texture360Array`))))
            (else
              (set `self.StaticMesh2_Mat` (- (`self.StaticMesh2_Mat`) 5))))
          (bind _returnvalue_3 (`KismetMaterialLibrary.CreateDynamicMaterialInstance` "/Game/Videos/UI_VID_IMAGE/IMage/360/M_anh360_Inst.M_anh360_Inst"))
          (`MaterialInstanceDynamic.SetTextureParameterValue` _returnvalue_3 "Image360" (`|GetArrayItem` (`self.Texture360Array`) (`self.StaticMesh2_Mat`)))
          (`PrimitiveComponent.SetMaterial` (`self.StaticMesh2`) 0 _returnvalue_3)
          (bind (_direction_6 _scale_6) (`Timeline|Timeline_15` :!via `PlayFromStart`)
            (:`Update`
              (`SceneComponent.SetWorldScale3D` (`self.StaticMesh2`) (`KismetMathLibrary.MakeVector` _scale_6 _scale_6 _scale_6)))))))
    (:`then_3`
      (bind (_direction_7 _scale_7) (`Timeline|Timeline_16` :!via `PlayFromStart`)
        (:`Update`
          (`SceneComponent.SetWorldScale3D` (`self.StaticMesh3`) (`KismetMathLibrary.MakeVector` _scale_7 _scale_7 _scale_7)))
        (:`Finished`
          (if (<= (`self.StaticMesh3_Mat`) 4)
            (set `self.StaticMesh3_Mat` (+ (- (`self.StaticMesh3_Mat`) 5) (`KismetArrayLibrary.Array_Length` (`self.Texture360Array`))))
            (else
              (set `self.StaticMesh3_Mat` (- (`self.StaticMesh3_Mat`) 5))))
          (bind _returnvalue_4 (`KismetMaterialLibrary.CreateDynamicMaterialInstance` "/Game/Videos/UI_VID_IMAGE/IMage/360/M_anh360_Inst.M_anh360_Inst"))
          (`MaterialInstanceDynamic.SetTextureParameterValue` _returnvalue_4 "Image360" (`|GetArrayItem` (`self.Texture360Array`) (`self.StaticMesh3_Mat`)))
          (`PrimitiveComponent.SetMaterial` (`self.StaticMesh3`) 0 _returnvalue_4)
          (bind (_direction_8 _scale_8) (`Timeline|Timeline_17` :!via `PlayFromStart`)
            (:`Update`
              (`SceneComponent.SetWorldScale3D` (`self.StaticMesh3`) (`KismetMathLibrary.MakeVector` _scale_8 _scale_8 _scale_8)))))))
    (:`then_4`
      (bind (_direction_9 _scale_9) (`Timeline|Timeline_18` :!via `PlayFromStart`)
        (:`Update`
          (`SceneComponent.SetWorldScale3D` (`self.StaticMesh4`) (`KismetMathLibrary.MakeVector` _scale_9 _scale_9 _scale_9)))
        (:`Finished`
          (if (<= (`self.StaticMesh4_Mat`) 4)
            (set `self.StaticMesh4_Mat` (+ (`KismetArrayLibrary.Array_Length` (`self.Texture360Array`)) (- (`self.StaticMesh4_Mat`) 5)))
            (else
              (set `self.StaticMesh4_Mat` (- (`self.StaticMesh4_Mat`) 5))))
          (bind _returnvalue_5 (`KismetMaterialLibrary.CreateDynamicMaterialInstance` "/Game/Videos/UI_VID_IMAGE/IMage/360/M_anh360_Inst.M_anh360_Inst"))
          (`MaterialInstanceDynamic.SetTextureParameterValue` _returnvalue_5 "Image360" (`|GetArrayItem` (`self.Texture360Array`) (`self.StaticMesh4_Mat`)))
          (`PrimitiveComponent.SetMaterial` (`self.StaticMesh4`) 0 _returnvalue_5)
          (bind (_direction_10 _scale_10) (`Timeline|Timeline_19` :!via `PlayFromStart`)
            (:`Update`
              (`SceneComponent.SetWorldScale3D` (`self.StaticMesh4`) (`KismetMathLibrary.MakeVector` _scale_10 _scale_10 _scale_10)))))))))

(fn `Off360Image`
  (bind _staticmesh1 (`self.StaticMesh1`))
  (`SceneComponent.SetVisibility` _staticmesh1 false false)
  (`SceneComponent.SetVisibility` (`self.StaticMesh2`) false false)
  (`SceneComponent.SetVisibility` (`self.StaticMesh3`) false false)
  (`SceneComponent.SetVisibility` (`self.StaticMesh4`) false false)
  (`SceneComponent.SetVisibility` (`self.StaticMesh`) false false)
  (`PrimitiveComponent.SetCollisionEnabled` _staticmesh1 "NoCollision")
  (`PrimitiveComponent.SetCollisionEnabled` (`self.StaticMesh2`) "NoCollision")
  (`PrimitiveComponent.SetCollisionEnabled` (`self.StaticMesh3`) "NoCollision")
  (`PrimitiveComponent.SetCollisionEnabled` (`self.StaticMesh4`) "NoCollision")
  (`PrimitiveComponent.SetCollisionEnabled` (`self.StaticMesh`) "NoCollision"))

(fn `On360Image`
  (bind _staticmesh1 (`self.StaticMesh1`))
  (`SceneComponent.SetVisibility` _staticmesh1 true false)
  (`SceneComponent.SetVisibility` (`self.StaticMesh2`) true false)
  (`SceneComponent.SetVisibility` (`self.StaticMesh3`) true false)
  (`SceneComponent.SetVisibility` (`self.StaticMesh4`) true false)
  (`SceneComponent.SetVisibility` (`self.StaticMesh`) true false)
  (`PrimitiveComponent.SetCollisionEnabled` _staticmesh1 "QueryAndPhysics")
  (`PrimitiveComponent.SetCollisionEnabled` (`self.StaticMesh2`) "QueryAndPhysics")
  (`PrimitiveComponent.SetCollisionEnabled` (`self.StaticMesh3`) "QueryAndPhysics")
  (`PrimitiveComponent.SetCollisionEnabled` (`self.StaticMesh4`) "QueryAndPhysics")
  (`PrimitiveComponent.SetCollisionEnabled` (`self.StaticMesh`) "QueryAndPhysics"))

(fn `UserConstructionScript`)