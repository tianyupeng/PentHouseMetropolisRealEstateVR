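; LeftUI is a VR menu actor whose widget floats above the player's left hand and yaws toward the camera each tick.
; On BeginPlay it creates a LeftUIMain widget linked to the MySoundAmbient actor, and each tick syncs collision to visibility.
; UIon shows it and clears media flags; UIOff hides it and UI_TV screens, resets sound, and ends image, video or 360 views.
; A timeline drives the widget's emissive glow.
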(event `self.ReceiveBeginPlay`
  (bind _outactors (`GameplayStatics.GetAllActorsOfClass` "/Game/Blueprints/MySoundAmbient.MySoundAmbient_C"))
  (for _array_element _outactors
    (set `self.MySoundMaster` _array_element))
  (bind _returnvalue (`|CreateWidget` "/Game/Blueprints/Widget/LeftUIMain.LeftUIMain_C" null false (`self.MySoundMaster`) self))
  (`WidgetComponent.SetWidget` (`self.Widget`) _returnvalue)
  (set `self.VRWidget` _returnvalue))

(event `self.ReceiveTick`
  (params (DeltaSeconds :type "Float (single-precision)"))
  (bind _widget (`self.Widget`))
  (bind _asvr_home (cast `/Game/Blueprints/VR_Home` (`GameplayStatics.GetPlayerPawn` 0) :!pure true))
  (`|ExecutionSequence`
    (:`then_0`
      (`self.K2_SetActorLocationAndRotation` (+ (`SceneComponent.K2_GetComponentLocation` (`/Game/Blueprints/VR_Home.LeftHand` _asvr_home)) (* (`self.GetActorUpVector` _asvr_home) 20.0)) (`KismetMathLibrary.MakeRotator` 0.0 0.0 (.yaw (`KismetMathLibrary.FindLookAtRotation` (`self.K2_GetActorLocation`) (`SceneComponent.K2_GetComponentLocation` (`/Game/Blueprints/VR_Home.Camera` _asvr_home)))))))
    (:`then_1`
      (if (`SceneComponent.bVisible` (`self.Widget`))
        (`PrimitiveComponent.SetCollisionEnabled` _widget "QueryOnly")
        (else
          (`PrimitiveComponent.SetCollisionEnabled` _widget "NoCollision"))))))

(event `AddUIEmissive`
  (params (in :type Boolean))
  (if in
    (bind (_direction _float) (`Timeline|time1` :!via `PlayFromStart` :!label _label)
      (:`Update`
        (`MaterialInstanceDynamic.SetScalarParameterValue` (`WidgetComponent.GetMaterialInstance` (`self.Widget`)) "Emissive" _float)))
    (else
      (goto _label :!via `Reverse`))))

(fn `UIOff`
  (bind _vrwidget (`self.VRWidget`))
  (bind _vrwidget_2 (`self.VRWidget`))
  (bind _widget (`self.Widget`))
  (bind _vrwidget_3 (`self.VRWidget`))
  (if (`/Game/Blueprints/Widget/LeftUIMain.360image?` _vrwidget_3)
    (`/Game/Blueprints/Widget/LeftUIMain.TurnOff360Mat` _vrwidget_3))
  (`PrimitiveComponent.SetCollisionEnabled` _widget "NoCollision")
  (`SceneComponent.SetVisibility` _widget false false)
  (bind _outactors (`GameplayStatics.GetAllActorsWithTag` "UI_TV"))
  (for _array_element _outactors
    (bind _asmy_ul_tv (cast `/Game/Blueprints/Object/MyUL_TV` _array_element))
    (bind _staticmesh (`/Game/Blueprints/Object/MyUL_TV.StaticMesh` _asmy_ul_tv))
    (`SceneComponent.SetVisibility` _staticmesh false false)
    (`PrimitiveComponent.SetCollisionEnabled` _staticmesh "NoCollision"))
  (`/Game/Blueprints/MySoundAmbient.SetSound` (`self.MySoundMaster`) "/Game/Sound/Etemal-Field.Etemal-Field")
  (if (or (`/Game/Blueprints/Widget/LeftUIMain.Video` _vrwidget_2) (`/Game/Blueprints/Widget/LeftUIMain.Image` _vrwidget_2))
    (`/Game/Blueprints/VR_Home.CinematicDisableView` (cast `/Game/Blueprints/VR_Home` (`GameplayStatics.GetPlayerPawn` 0) :!pure true))
    (set `/Game/Blueprints/Widget/LeftUIMain.Image` false _vrwidget)
    (set `/Game/Blueprints/Widget/LeftUIMain.Video` false _vrwidget)
    (set `/Game/Blueprints/Widget/LeftUIMain.360image?` false _vrwidget)))

(fn `UIon`
  (bind _vrwidget (`self.VRWidget`))
  (bind _widget (`self.Widget`))
  (`PrimitiveComponent.SetCollisionEnabled` _widget "QueryOnly")
  (`SceneComponent.SetVisibility` _widget true false)
  (set `/Game/Blueprints/Widget/LeftUIMain.Image` false _vrwidget)
  (set `/Game/Blueprints/Widget/LeftUIMain.Video` false _vrwidget)
  (set `/Game/Blueprints/Widget/LeftUIMain.360image?` false _vrwidget))

(fn `UserConstructionScript`)